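; BOLABP is a ball actor that gets launched toward an aim target when another actor overlaps it.
; The construction script caches the first PlanoDaMiraBP found in the level as Alvo.
; On overlap, the Bola component receives a fixed-strength, mass-dependent impulse along the normalized direction from itself to the AlvoCone component of Alvo.
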(event Collision|EventActorBeginOverlap
  (params (OtherActor :type Actor%20Object%20Reference))
  (bind _bola (Variables|Default|Getbola))
  (Physics|AddImpulse _bola (* (Math|Vector|Normalize (Math|Vector|GetUnitDirection(Vector) (Transformation|GetWorldLocation _bola) (Transformation|GetWorldLocation (Variables|/Game/PlanoDaMiraBP.PlanoDaMiraBP_C|Getalvo%20cone (Variables|Default|GetAlvo))))) 1.5e+03) "None" false))

(fn ConstructionScript
  (bind _outactors (Actor|GetAllActorsOfClass "/Game/PlanoDaMiraBP.PlanoDaMiraBP_C"))
  (Variables|Default|SetAlvo (Utilities|Array|Get(acopy) _outactors)))